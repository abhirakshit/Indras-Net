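; BP_ThoughtLT is a debug-drawn prototype of a "thought" ray that bounces around inside a sphere centered on the actor.
; From BeginPlay, TraceEffect calculates the sphere exit point and reflection mathematically, draws a line trace, then re-calls itself after a delay.
; A separate ThoughtStart path, not called here, bounces off real trace hits using impact normals.
; Print messages report points, hits and failures.
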(event OnComponentHit(Sphere)
  (params (HitComponent :type Primitive%20Component%20Object%20Reference) (OtherActor :type Actor%20Object%20Reference) (OtherComp :type Primitive%20Component%20Object%20Reference) (NormalImpulse :type Vector :default "0, 0, 0") (Hit :type Hit%20Result%20Structure%20%28by%20ref%29))
  (Development|PrintText "Colission |Sphere hit"))

(event Custom|TraceAndReflectRay
  (params (StartLocation :type Vector) (Direction :type Vector))
  (bind _outhit (CallFunction|LineTraceforReflection StartLocation Direction))
  (if (.bBlockingHit (Collision|BreakHitResult _outhit))
    (Development|PrintText "Hit")
    (bind _reflecteddirection (CallFunction|CalculateReflectionDirection _outhit Direction))
    (Utilities|FlowControl|Delay 1.0)
    (CallFunction|TraceandReflectRay (.ImpactPoint (Collision|BreakHitResult _outhit)) _reflecteddirection)
    (else
      (Development|PrintText "Nooooo"))))

(event Custom|TraceEffect
  (params (startPoint :type Vector) (direction :type Vector))
  (bind _returnvalue (Transformation|GetActorLocation))
  (bind _radius (Variables|Default|GetRadius))
  (Utilities|FlowControl|Sequence
    (:then_0
      (Variables|Default|SetStartPoint startPoint))
    (:then_1
      (if (.bSuccessful (Class|ThoughtCoordinateFunctions|CalculateIntersectionPoint _returnvalue _radius (Variables|Default|GetStartPoint) direction))
        (Variables|Default|SetEndPoint (.ReturnValue (Class|ThoughtCoordinateFunctions|CalculateIntersectionPoint _returnvalue _radius (Variables|Default|GetStartPoint) direction)))
        (Collision|LineTraceByChannel (Variables|Default|GetStartPoint) (Variables|Default|GetEndPoint) "TraceTypeQuery1" true 0 "ForDuration")
        (Development|PrintText (Utilities|Text|FormatText "start: {start}, end: {end}" (Utilities|Text|ToText(String) (Variables|Default|GetStartPoint)) (Utilities|Text|ToText(String) (Variables|Default|GetEndPoint))) true true "(R=0.000000,G=0.660000,B=1.000000,A=1.000000)" 1e+01)
        (Utilities|FlowControl|Delay 1.0)
        (CallFunction|TraceEffect (Variables|Default|GetEndPoint) (Variables|Default|GetReflectedDirection))
        (else
          (Development|PrintText "Error calculating hit point"))))
    (:then_2
      (if (.bSuccessful (Class|ThoughtCoordinateFunctions|CalculateReflection _returnvalue _radius (Variables|Default|GetStartPoint) direction (Variables|Default|GetReflectionCoefficient)))
        (Variables|Default|SetReflectedDirection (.ReflectedDirection (Class|ThoughtCoordinateFunctions|CalculateReflection _returnvalue _radius (Variables|Default|GetStartPoint) direction (Variables|Default|GetReflectionCoefficient))))
        (else
          (Development|PrintText "Invalif Reflection"))))))

(event Custom|ThoughtStart
  (bind _output_get (Variables|Default|SetStartPoint (Transformation|GetActorLocation)))
  (bind _output_get_2 (Variables|Default|SetRayDirection (Math|Random|RandomUnitVector)))
  (CallFunction|TraceandReflectRay _output_get _output_get_2))

(event EventBeginPlay
  (bind _output_get (Variables|Default|SetStartPoint (+ (Transformation|GetActorLocation) (Math|Vector|MakeVector (Math|Random|RandomFloatinRange 5.0 15.0) (Math|Random|RandomFloatinRange 5.0 15.0) (Math|Random|RandomFloatinRange 5.0 15.0)))))
  (bind _output_get_2 (Variables|Default|SetRayDirection (Math|Random|RandomUnitVector)))
  (CallFunction|TraceEffect _output_get _output_get_2))

(fn ConstructionScript)

(fn CalculateReflectionDirection
  (params (HitResult :type Hit%20Result%20Structure) (Direction :type Vector))
  (return (Math|Vector|GetReflectionVector Direction (.ImpactNormal (Collision|BreakHitResult HitResult)))))

(fn LineTraceforReflection
  (params (StartLocation :type Vector) (Direction :type Vector))
  (bind (_outhit _returnvalue) (Collision|LineTraceByChannel StartLocation (+ StartLocation (* Direction 1e+04)) "TraceTypeQuery1" true 0 "ForDuration"))
  (if _returnvalue
    (Development|PrintText (Utilities|Text|FormatText "Hit {t1}, {out}" _returnvalue (Utilities|Text|ToText(String) (.ImpactPoint (Collision|BreakHitResult _outhit)))))
    (return _outhit)
    (else
      (Development|PrintText "Miss Ray trace"))))

(fn CreateInternalSphereCollision)