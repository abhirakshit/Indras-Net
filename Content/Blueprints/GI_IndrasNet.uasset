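; GI_IndrasNet is the game instance for IndrasNet, holding the loaded save game and vessel data.
; A load event reads the "default" slot into SavedGame, and another event stores the current vessel's data.
; Getters expose the current vessel, the SavedVessels collection and the instance itself.
; The load does not copy anything into SavedVessels, and nothing here writes to the save.
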(event EventLoadSavedGameData
  (bind _returnvalue (SaveGame|LoadGamefromSlot "default"))
  (Variables|Default|SetsavedGame _returnvalue))

(event EventSetCurrentVesselData
  (params (currentVessel :type BP%20Vessel%20Data%20Struct%20Structure))
  (Variables|Default|SetcurrentVesselData currentVessel))

(fn GetAllSavedVesselData
  (return (Variables|Default|GetsavedVessels)))

(fn GetCurrentVesselData
  (return (Variables|Default|GetcurrentVesselData)))

(fn SetGameInstanceRef
  (return self))