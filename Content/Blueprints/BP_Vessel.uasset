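; BP_Vessel is a layered glass orb actor that visualizes a character's six personality traits and emotional state.
; Setup takes a data struct, mapping traits onto dynamic material parameters, shell scale, rotation, core offset and spawned imperfections; Agreeableness is only stored.
; Emotion updates colour the core by blending the top two DT_EmotionColors hues, intensity-scaled, using square-root RGB interpolation.
; startThoughtBeam spawns a Niagara effect; CreateThoughtBeam and collision events are debug stubs.
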(event OnComponentHit(CollisionSphere)
  (params (HitComponent :type Primitive%20Component%20Object%20Reference) (OtherActor :type Actor%20Object%20Reference) (OtherComp :type Primitive%20Component%20Object%20Reference) (NormalImpulse :type Vector :default "0, 0, 0") (Hit :type Hit%20Result%20Structure%20%28by%20ref%29))
  (Development|PrintText "Hit collision"))

(event OnComponentBeginOverlap(CollisionSphere)
  (params (OverlappedComponent :type Primitive%20Component%20Object%20Reference) (OtherActor :type Actor%20Object%20Reference) (OtherComp :type Primitive%20Component%20Object%20Reference) (OtherBodyIndex :type Integer) (bFromSweep :type Boolean) (SweepResult :type Hit%20Result%20Structure%20%28by%20ref%29))
  (Development|PrintText "overlap collision"))

(event OnComponentHit(OuterShell_O)
  (params (HitComponent :type Primitive%20Component%20Object%20Reference) (OtherActor :type Actor%20Object%20Reference) (OtherComp :type Primitive%20Component%20Object%20Reference) (NormalImpulse :type Vector :default "0, 0, 0") (Hit :type Hit%20Result%20Structure%20%28by%20ref%29))
  (Development|PrintText "Hit Mesh"))

(event OnClicked(OuterShell_O)
  (params (TouchedComponent :type Primitive%20Component%20Object%20Reference) (ButtonPressed :type Key%20Structure))
  (Development|PrintText "Click Mesh"))

(event Custom|startThoughtBeam
  (bind _thoughtstartpoint (Variables|Default|GetThoughtStartPoint))
  (bind _returnvalue (Transformation|GetWorldTransform _thoughtstartpoint))
  (Development|PrintText (Utilities|Text|ToText(String) (.BoxExtent (Collision|GetComponentBounds (Variables|Default|GetOuterShell_O)))) true true "(R=0.000000,G=0.660000,B=1.000000,A=1.000000)" 1e+01)
  (Niagara|SpawnSystematLocation "/Game/Niagara/NS_Thought.NS_Thought" (.location _returnvalue) (.rotation _returnvalue)))

(event EventBeginPlay)

(fn ConstructionScript
  (Utilities|FlowControl|Sequence
    (:then_0
      (bind _returnvalue (Rendering|Material|CreateDynamicMaterialInstance (Variables|Default|GetInnerSphere) 0 "/Game/Assets/Instances/MI_MagicOrbInner.MI_MagicOrbInner" "None" :!class /Script/Engine.PrimitiveComponent))
      (Variables|Default|SetMI_InnerSphere _returnvalue))
    (:then_1
      (bind _returnvalue_2 (Rendering|Material|CreateDynamicMaterialInstance (Variables|Default|GetOuterShell_I) 0 "/Game/Assets/Instances/MI_TransparentGlass.MI_TransparentGlass" "None" :!class /Script/Engine.PrimitiveComponent))
      (Variables|Default|SetMI_OuterInnerSphere _returnvalue_2))
    (:then_2
      (bind _returnvalue_3 (Rendering|Material|CreateDynamicMaterialInstance (Variables|Default|GetOuterShell_O) 0 "/Game/Assets/Instances/MI_TransparentGlass.MI_TransparentGlass" "None" :!class /Script/Engine.PrimitiveComponent))
      (Variables|Default|SetMI_OuterSphere _returnvalue_3))))

(fn UpdateHonesty
  (params (honesty :type Float%20%28double-precision%29))
  ;[1 1 1] Outer shell material change: roughness
  (bind _output_get (Variables|Default|Sethonesty honesty))
  (Utilities|FlowControl|Sequence
    (:then_0
      (Rendering|Material|SetScalarParameterValue (Variables|Default|GetMI_OuterSphere) "Roughness" (Math|Float|Lerp 5e+01 1.0 (Math|Float|NormalizetoRange _output_get 1.0 5.0)) :!class /Script/Engine.MaterialInstanceDynamic))
    (:then_1
      (CallFunction|UpdateImperfections (Math|Conversions|ToInteger(Byte) (Class|KismetMathLibrary|FFloor64 (Math|Float|Lerp 8.0 0.0 (Math|Float|NormalizetoRange _output_get 1.0 5.0)))) (Math|Float|Lerp 5.0 15.0 (Math|Float|NormalizetoRange _output_get 1.0 5.0))))))

(fn Setup
  (params (dataStruct :type BP%20Vessel%20Data%20Struct%20Structure))
  (bind (_name _desc _hnsty _emot _extra _agree _consc _open _id) (Utilities|Struct|BreakBP_VesselDataStruct dataStruct))
  (Utilities|FlowControl|Sequence
    (:then_0
      (CallFunction|UpdateAgreeableness _agree))
    (:then_1
      (CallFunction|UpdateHonesty _hnsty))
    (:then_2
      (CallFunction|UpdateExtraversion _extra))
    (:then_3
      (CallFunction|UpdateOpenness _open))
    (:then_4
      (Variables|Default|Setname _name))
    (:then_5
      (Variables|Default|Setdescription _desc))
    (:then_6
      (Variables|Default|Setid _id))
    (:then_7
      (CallFunction|UpdateEmotionality _emot))
    (:then_8
      (CallFunction|UpdateConscientiousness _consc))))

(fn UpdateOpenness
  (params (openness :type Float%20%28double-precision%29))
  (bind _output_get (Variables|Default|Setopenness openness))
  (Utilities|FlowControl|Sequence
    (:then_0
      ;[1 1 1] Inner shell change to showcase shell thickness
      (Transformation|SetRelativeScale3D (Variables|Default|GetOuterShell_I) (Math|Conversions|ToVector(Float) (Math|Float|Lerp 0.8 0.98 (Math|Float|NormalizetoRange _output_get 1.0 5.0)))))
    (:then_1
      ;[1 1 1] Outer shell material change to showcase shell opacity
      (Rendering|Material|SetScalarParameterValue (Variables|Default|GetMI_OuterSphere) "Opacity In" (Math|Float|Lerp 0.7 0.0 (Math|Float|NormalizetoRange _output_get 1.0 5.0)) :!class /Script/Engine.MaterialInstanceDynamic)
      (Rendering|Material|SetScalarParameterValue (Variables|Default|GetMI_InnerSphere) "Opacity In" (Math|Float|Lerp 0.7 0.0 (Math|Float|NormalizetoRange _output_get 1.0 5.0)) :!class /Script/Engine.MaterialInstanceDynamic))))

(fn UpdateExtraversion
  (params (extraversion :type Float%20%28double-precision%29))
  ;[1 1 1] Inner shell material change to showcase shell brightness
  (bind _output_get (Variables|Default|Setextraversion extraversion))
  (Rendering|Material|SetScalarParameterValue (Variables|Default|GetMI_InnerSphere) "Inner_Brightness" (Math|Float|Lerp 5.0 2e+01 (Math|Float|NormalizetoRange _output_get 1.0 5.0)) :!class /Script/Engine.MaterialInstanceDynamic))

(fn UpdateEmotionality
  (params (emotionality :type Float%20%28double-precision%29))
  (bind _mi_innersphere (Variables|Default|GetMI_InnerSphere))
  ;[1 1 1] Outer shell material change: roughness
  (bind _output_get (Variables|Default|Setemotionality emotionality))
  (Utilities|FlowControl|Sequence
    (:then_0
      (Rendering|Material|SetScalarParameterValue _mi_innersphere "SkyStar_Brightness" (Math|Float|Lerp 1.0 3e+01 (Math|Float|NormalizetoRange _output_get 1.0 5.0)) :!class /Script/Engine.MaterialInstanceDynamic))
    (:then_1
      (Rendering|Material|SetScalarParameterValue _mi_innersphere "Tex_Speed" (Math|Float|Lerp 0.3 0.9 (Math|Float|NormalizetoRange _output_get 1.0 5.0)) :!class /Script/Engine.MaterialInstanceDynamic))
    (:then_2
      (Rendering|Material|SetScalarParameterValue _mi_innersphere "Tex_PannerX" (Math|Float|Lerp 0.0 0.5 (Math|Float|NormalizetoRange _output_get 1.0 5.0)) :!class /Script/Engine.MaterialInstanceDynamic))
    (:then_3
      (Rendering|Material|SetScalarParameterValue _mi_innersphere "Tex_PannerX" (Math|Float|Lerp 0.0 0.5 (Math|Float|NormalizetoRange _output_get 1.0 5.0)) :!class /Script/Engine.MaterialInstanceDynamic))))

(fn GetVesselDataStruct
  (return (Utilities|Struct|MakeBP_VesselDataStruct (Variables|Default|Getname) (Variables|Default|Getdescription) (Variables|Default|Gethonesty) (Variables|Default|Getemotionality) (Variables|Default|Getextraversion) (Variables|Default|Getagreeableness) (Variables|Default|Getconscientiousness) (Variables|Default|Getopenness) (Variables|Default|Getid))))

(fn UpdateImperfections
  (params (count :type Integer) (opacity :type Float%20%28double-precision%29))
  (bind _imperfections (Variables|Default|Getimperfections))
  (bind _imperfections_2 (Variables|Default|Getimperfections))
  (bind _returnvalue (Utilities|Array|Length _imperfections_2))
  (Utilities|FlowControl|Sequence
    (:then_0
      ;[1 1 1] Set Count, Opacity and if imperfections need to be added or removed
      (LocalVariables|SetlCount count)
      (LocalVariables|SetlOpacity opacity))
    (:then_1
      (LocalVariables|SetaddImperfection (> count _returnvalue)))
    (:then_2
      (LocalVariables|Setdiff (Math|Integer|Absolute(Integer) (- (LocalVariables|GetlCount) _returnvalue))))
    (:then_3
      (if (LocalVariables|GetaddImperfection)
        (for _index (range 0 (LocalVariables|Getdiff))
          (bind _returnvalue_2 (Game|SpawnActorfromClass "/Game/Blueprints/BP_Imperfection.BP_Imperfection_C" (Math|Transform|MakeTransform (+ (Transformation|GetActorLocation) (* (Math|Random|RandomUnitVector) (Math|Random|RandomFloatinRange 8e+01 1.5e+02))) "0, 0, 0" (Math|Conversions|ToVector(Float) (Math|Random|RandomFloatinRange 0.4 1.0))) "Undefined" 0 0))
          (Utilities|Array|AddUnique (Variables|Default|Getimperfections) _returnvalue_2))
        (elif (> (LocalVariables|Getdiff) 0)
          (Actor|DestroyActor (Utilities|Array|Get(acopy) _imperfections))
          (Utilities|Array|RemoveIndex _imperfections))))))

(fn UpdateAgreeableness
  (params (agreeableness :type Float%20%28double-precision%29))
  (Variables|Default|Setagreeableness agreeableness))

(fn UpdateConscientiousness
  (params (conscientiousness :type Float%20%28double-precision%29))
  (bind _output_get (Variables|Default|Setconscientiousness conscientiousness))
  (Utilities|FlowControl|Sequence
    (:then_0
      (Variables|/Script/Engine.RotatingMovementComponent|SetRotationRate (Variables|Default|GetRotatingMovement) (Math|Rotator|MakeRotator (Math|Float|Lerp 22.5 5.0 (Math|Float|NormalizetoRange _output_get 0.0 5.0)) (Math|Float|Lerp 22.5 5.0 (Math|Float|NormalizetoRange _output_get 0.0 5.0)) (Math|Float|Lerp 22.5 5.0 (Math|Float|NormalizetoRange _output_get 0.0 5.0)))))
    (:then_1
      (Transformation|SetWorldLocation (Variables|Default|GetInnerSphere) (+ (Math|Vector|MakeVector (Math|Float|Lerp 5e+01 0.0 (Math|Float|NormalizetoRange _output_get 0.0 5.0)) (Math|Float|Lerp 5e+01 0.0 (Math|Float|NormalizetoRange _output_get 0.0 5.0)) (Math|Float|Lerp 5e+01 0.0 (Math|Float|NormalizetoRange _output_get 0.0 5.0))) (Transformation|GetActorLocation)) false false))))

(fn CreateThoughtBeam
  (Development|PrintText "Start Beam")
  (bind _index (Utilities|FlowControl|ForLoopwithBreak 0 (Variables|Default|Getdistance))))

(fn UpdateEmotion
  (params (value :type Float%20%28double-precision%29) (emotionTxt :type String))
  (Utilities|Map|Add (Variables|Default|GetemotionalState) emotionTxt value)
  (CallFunction|UpdateInnerSphereColor))

(fn UpdateInnerSphereColor
  (bind _emotionalstate (Variables|Default|GetemotionalState))
  (bind _mi_innersphere (Variables|Default|GetMI_InnerSphere))
  ;[1 1 1] Sort and find top 2 emotions
  (bind _sorted_map (Class|SortingArray|SortMapbyValue (Variables|Default|GetemotionalState) true))
  (bind _keys (Utilities|Map|Keys _sorted_map))
  (bind _returnvalue (Utilities|GetDataTableRow "/Game/Library/DT_EmotionColors.DT_EmotionColors" (Utilities|String|StringToName (Utilities|Array|Get(acopy) _keys)))
    (:then
      (bind _returnvalue_2 (Utilities|GetDataTableRow "/Game/Library/DT_EmotionColors.DT_EmotionColors" (Utilities|String|StringToName (Utilities|Array|Get(acopy) _keys 1)))
        (:then
          (bind _newcolor (CallFunction|BlendColors (Class|KismetMathLibrary|HSVtoRGB (.H (Math|Color|RGBtoHSV(LinearColor) (Utilities|Struct|MakeLinearColor (.r (Utilities|Struct|BreakDS_EmotionColor _returnvalue)) (.g (Utilities|Struct|BreakDS_EmotionColor _returnvalue)) (.b (Utilities|Struct|BreakDS_EmotionColor _returnvalue)) (.a (Utilities|Struct|BreakDS_EmotionColor _returnvalue))))) (Math|Float|Lerp 0.5 0.9 (Math|Float|NormalizetoRange (.Value (Utilities|Map|Find _emotionalstate (Utilities|Array|Get(acopy) _keys))) 1.0 5.0)) (Math|Float|Lerp 0.5 0.9 (Math|Float|NormalizetoRange (.Value (Utilities|Map|Find _emotionalstate (Utilities|Array|Get(acopy) _keys))) 1.0 5.0)) 1.0) (Class|KismetMathLibrary|HSVtoRGB (.H (Math|Color|RGBtoHSV(LinearColor) (Utilities|Struct|MakeLinearColor (.r (Utilities|Struct|BreakDS_EmotionColor _returnvalue_2)) (.g (Utilities|Struct|BreakDS_EmotionColor _returnvalue_2)) (.b (Utilities|Struct|BreakDS_EmotionColor _returnvalue_2)) (.a (Utilities|Struct|BreakDS_EmotionColor _returnvalue_2))))) (Math|Float|Lerp 0.5 0.9 (Math|Float|NormalizetoRange (.Value (Utilities|Map|Find _emotionalstate (Utilities|Array|Get(acopy) _keys 1))) 1.0 5.0)) (Math|Float|Lerp 0.5 0.9 (Math|Float|NormalizetoRange (.Value (Utilities|Map|Find _emotionalstate (Utilities|Array|Get(acopy) _keys 1))) 1.0 5.0)) 1.0) 0.2))
          (Rendering|Material|SetVectorParameterValue _mi_innersphere "Inner_Color" _newcolor :!class /Script/Engine.MaterialInstanceDynamic)
          (Rendering|Material|SetVectorParameterValue _mi_innersphere "Outline_Color" _newcolor :!class /Script/Engine.MaterialInstanceDynamic))
        (:RowNotFound
          (Development|PrintText (Utilities|Text|FormatText "Error: 1: {e1}, 2: {e2}" (Utilities|Array|Get(acopy) _keys) (Utilities|Array|Get(acopy) _keys 1)) true true "(R=1.000000,G=0.149752,B=0.311974,A=1.000000)" :!label _label))))
    (:RowNotFound
      (goto _label))))

(fn BlendColors
  (params (c1 :type Linear%20Color%20Structure) (c2 :type Linear%20Color%20Structure) (blendPoint :type Float%20%28double-precision%29))
  (bind _output_get (LocalVariables|Setcolor1 c1))
  (bind _output_get_2 (LocalVariables|Setcolor2 c2))
  (LocalVariables|Sett blendPoint)
  (return (Math|Color|MakeColor (Math|Float|Sqrt (+ (* (- 1.0 (LocalVariables|Gett)) (Math|Float|Square (.r (LocalVariables|Getcolor1)))) (* (LocalVariables|Gett) (Math|Float|Square (.r (LocalVariables|Getcolor2)))))) (Math|Float|Sqrt (+ (* (- 1.0 (LocalVariables|Gett)) (Math|Float|Square (.g (LocalVariables|Getcolor1)))) (* (LocalVariables|Gett) (Math|Float|Square (.g (LocalVariables|Getcolor2)))))) (Math|Float|Sqrt (+ (* (- 1.0 (LocalVariables|Gett)) (Math|Float|Square (.b (LocalVariables|Getcolor1)))) (* (LocalVariables|Gett) (Math|Float|Square (.b (LocalVariables|Getcolor2)))))) (+ (* (- 1.0 (LocalVariables|Gett)) (.a (LocalVariables|Getcolor1))) (* (LocalVariables|Gett) (.a (LocalVariables|Getcolor2)))))))