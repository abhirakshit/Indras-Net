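; GM_IndrasNet is a game mode Blueprint that spawns the current vessel and keeps a reference to it.
; The SpawnVesselWithData event reads the current vessel data from the game instance and passes it into a scaled-up BP_Vessel spawned at a fixed raised location.
; Getter functions expose the stored vessel and the game mode itself to other Blueprints.
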(event Custom|SpawnVesselWithData
  (bind _gameinstance (Class|INTGameInstance|SetGameInstanceRef(Message) (Game|GetGameInstance)))
  (bind _output_get (Variables|Default|SetGame%20Instance _gameinstance))
  (bind _currentvesseldata (Default|GetCurrentVesselData _output_get))
  (bind _returnvalue (Game|SpawnActorfromClass :Class "/Game/Blueprints/BP_Vessel.BP_Vessel_C" :SpawnTransform (Math|Transform|MakeTransform "0.000000,0.000000,400.000000" "0, 0, 0" "2.000000,2.000000,2.000000") :CollisionHandlingOverride "AdjustIfPossibleButAlwaysSpawn" :dataStruct _currentvesseldata :Instigator 0))
  (Variables|Default|SetVesselBP _returnvalue))

(fn ConstructionScript)

(fn GetCurrentVesselBP
  (return (Variables|Default|GetVesselBP)))

(fn SetGameModeRef
  (return self))