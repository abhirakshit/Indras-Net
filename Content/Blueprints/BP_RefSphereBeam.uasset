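; BP_RefSphereBeam is a debug-style actor that bounces a beam between surfaces from a fixed start point, spawning NS_Thought Niagara effects along the path.
; On BeginPlay it spawns an effect at the origin point and starts SpawnReflectedBeam, which line-traces on Visibility with debug drawing.
; Each hit spawns an effect oriented along the reflection vector, then recurses after a one-second delay until a trace misses, printing debug text.
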(event Custom|SpawnReflectedBeam
  (params (StartLocation :type Vector) (Direction :type Vector))
  (bind _outhit (CallFunction|LineTraceforReflection StartLocation Direction))
  (if (.bBlockingHit (Collision|BreakHitResult _outhit))
    (bind _reflecteddirection (CallFunction|CalculateReflectionDirection _outhit Direction))
    (Niagara|SpawnSystematLocation "/Game/Niagara/NS_Thought.NS_Thought" (.ImpactPoint (Collision|BreakHitResult _outhit)) (Math|Rotator|MakeRotfromX _reflecteddirection))
    (Utilities|FlowControl|Delay 1.0)
    (CallFunction|SpawnReflectedBeam (.ImpactPoint (Collision|BreakHitResult _outhit)) _reflecteddirection)
    (Development|PrintText (Utilities|Text|FormatText "{loc}, {dir}" (Utilities|Text|ToText(String) (.ImpactPoint (Collision|BreakHitResult _outhit))) (Utilities|Text|ToText(String) _reflecteddirection)))
    (else
      (Development|PrintText "No sphere hit"))))

(event EventBeginPlay
  (bind _returnvalue (Math|Vector|MakeVector 0.0 0.0 2e+02))
  (Utilities|FlowControl|Sequence
    (:then_0
      (Niagara|SpawnSystematLocation "/Game/Niagara/NS_Thought.NS_Thought" _returnvalue))
    (:then_1
      (CallFunction|SpawnReflectedBeam _returnvalue (Math|Vector|MakeVector 0.0 1.0 0.0)))))

(fn ConstructionScript)

(fn LineTraceforReflection
  (params (StartLocation :type Vector) (Direction :type Vector))
  (bind (_outhit _returnvalue) (Collision|LineTraceByChannel StartLocation (+ (* Direction 1e+04) StartLocation) "TraceTypeQuery1" false 0 "ForDuration"))
  (Development|PrintText (Utilities|Text|FormatText "Hit {t1}, {out}" _returnvalue (Utilities|Text|ToText(String) (.ImpactPoint (Collision|BreakHitResult _outhit)))))
  (return _outhit))

(fn CalculateReflectionDirection
  (params (HitResult :type Hit%20Result%20Structure) (Direction :type Vector))
  (return (Math|Vector|GetReflectionVector Direction (.ImpactNormal (Collision|BreakHitResult HitResult)))))